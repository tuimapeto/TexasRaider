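; Deputy enemy character that fights with a revolver attached to its hand socket at BeginPlay.
; Attack sets the AnimBP targeting pose, then fires a bullet from the revolver's arrow with sound and muzzle flash.
; Damage lowers health and flags IsDead, bullet hits spawn blood, and externally callable functions handle death, healing and walk speed.
; Timed question and exclamation markers follow overhead on Tick, turned toward the player camera, with exclamation taking priority.
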(event OnComponentHit(CapsuleComponent)
  (params (HitComponent :type Primitive%20Component%20Object%20Reference) (OtherActor :type Actor%20Object%20Reference) (OtherComp :type Primitive%20Component%20Object%20Reference) (NormalImpulse :type Vector :default "0, 0, 0") (Hit :type Hit%20Result%20Structure%20%28by%20ref%29))
  ;[0.15 0.15 0.15 0.5] Blood spawn
  (Utilities|Casting|CastToBP_Bullet OtherActor)
  (bind _returnvalue (Niagara|SpawnSystematLocation "/Game/VFX/sA_SplatterofbloodFx/Fx/PreShaded_Blood_Alternatives/NS_PreShadedBlood_2.NS_PreShadedBlood_2" (.location Hit)))
  (Utilities|FlowControl|Delay 2.0))

(event Custom|Attack
  ;[0.15 0.15 0.15 0.5] Attack Stance
  (bind _asanim_bp_deputy (Utilities|Casting|CastToAnimBP_Deputy (Components|SkeletalMesh|GetAnimInstance (Variables|Character|GetMesh))))
  (Variables|/Game/Enemies/Deputy/AnimBP_Deputy.AnimBP_Deputy_C|SetisTargeting? _asanim_bp_deputy true)
  (Utilities|FlowControl|Delay 0.3)
  (CallFunction|FireWeapon))

(event Custom|StopAttack
  ;[0.15 0.15 0.15 0.5] Attack Stance
  (bind _asanim_bp_deputy (Utilities|Casting|CastToAnimBP_Deputy (Components|SkeletalMesh|GetAnimInstance (Variables|Character|GetMesh))))
  (Variables|/Game/Enemies/Deputy/AnimBP_Deputy.AnimBP_Deputy_C|SetisTargeting? _asanim_bp_deputy false))

(event Custom|FireWeapon
  (bind _therevolver (Variables|Default|GetTheRevolver))
  (bind _returnvalue (Actor|GetComponentbyClass _therevolver "/Script/Engine.ArrowComponent"))
  (bind _returnvalue_2 (Game|SpawnActorfromClass "/Game/BluePrints/BP_BulletBase.BP_BulletBase_C" (Math|Conversions|ToTransform(Vector) (Transformation|GetActorLocation)) "Undefined" "MultiplyWithRoot" 0 0))
  (Transformation|SetActorLocation _returnvalue_2 (Transformation|GetWorldLocation _returnvalue) false false)
  (Transformation|SetActorRotation _returnvalue_2 (Transformation|GetWorldRotation _returnvalue))
  (Audio|PlaySoundatLocation "/Game/Audio/single-pistol-gunshot-33-37187.single-pistol-gunshot-33-37187" (Transformation|GetActorLocation) "0, 0, 0" 1.0 1.0 0.0 0 0 0 0)
  (bind _returnvalue_3 (Niagara|SpawnSystemAttached "/Game/VFX/Muzzle_Flash/FX/NS_Muzzle_Flash05.NS_Muzzle_Flash05" (Actor|GetComponentbyClass (Variables|Default|GetTheRevolver) "/Script/Engine.ArrowComponent") "None" "0, 0, 0" "0, 0, 0" "KeepRelativeOffset" false))
  (Utilities|FlowControl|Delay 0.6)
  (Components|DestroyComponent _returnvalue_3))

(event Custom|StopHeal
  ;[0.15 0.15 0.15 0.5] Stop Heal
  (Utilities|FlowControl|Delay 5.0)
  (bind _asanim_bp_deputy (Utilities|Casting|CastToAnimBP_Deputy (Components|SkeletalMesh|GetAnimInstance (Variables|Character|GetMesh))))
  (Variables|/Game/Enemies/Deputy/AnimBP_Deputy.AnimBP_Deputy_C|SetisHealing? _asanim_bp_deputy false))

(event Custom|OnActorHit_Event
  (params (SelfActor :type Actor%20Object%20Reference) (OtherActor :type Actor%20Object%20Reference) (NormalImpulse :type Vector) (Hit :type Hit%20Result%20Structure%20%28by%20ref%29))
  ;[0.15 0.15 0.15 0.5] Take damage
)

(event Custom|DeleteQuestionmark
  ;[0.15 0.15 0.15 0.5] Question Mark Deletion
  (Utilities|Time|SetTimerbyEvent (delegate Custom|QuestionDeleteTimer) 3.0)
  (Variables|Default|SetfaceCamera true))

(event Custom|QuestionDeleteTimer
  (bind _questionmark (Variables|Default|GetQuestionMark))
  ;[0.15 0.15 0.15 0.5] Question Mark Deletion
  (Utilities|IsValid _questionmark
    (:Is%20Valid
      (Actor|DestroyActor _questionmark))))

(event Custom|DeleteExclamationMark
  (bind _exclamationmark (Variables|Default|GetExclamationMark))
  ;[0.15 0.15 0.15 0.5] Excl Mark Delete
  (Utilities|FlowControl|Delay 3.0)
  (Utilities|IsValid _exclamationmark
    (:Is%20Valid
      (Actor|DestroyActor _exclamationmark))))

(event Custom|TranslateExclMark
  ;[0.15 0.15 0.15 0.5] Excl Mark face cam
  (Utilities|IsValid (Variables|Default|GetExclamationMark)
    (:Is%20Valid
      (Transformation|SetActorLocation (Variables|Default|GetExclamationMark) (+ (Transformation|GetActorLocation) (Math|Vector|MakeVector 0.0 0.0 1.5e+02)) false false))))

(event Custom|PreferExclamationMark
  ;[0.15 0.15 0.15 0.5] Prefer Exclamation
  (Utilities|IsValid (Variables|Default|GetQuestionMark)
    (:Is%20Valid
      (Utilities|IsValid (Variables|Default|GetExclamationMark)
        (:Is%20Valid
          (Actor|DestroyActor (Variables|Default|GetQuestionMark)))))))

(event EventBeginPlay
  ;[0.15 0.15 0.15 0.5] Spawn Weapon
  (bind _returnvalue (Game|SpawnActorfromClass "/Game/BluePrints/BP_Revolver.BP_Revolver_C" (Math|Conversions|ToTransform(Vector) (Transformation|GetActorLocation)) "Undefined" "MultiplyWithRoot" 0 0))
  (Variables|Default|SetTheRevolver _returnvalue)
  (Transformation|AttachComponentToComponent _returnvalue (Variables|Character|GetMesh) "Deputy_Socket" "SnapToTarget" "SnapToTarget" "KeepRelative" true))

(event Collision|EventActorBeginOverlap
  (params (OtherActor :type Actor%20Object%20Reference)))

(event EventTick
  (params (DeltaSeconds :type Float%20%28single-precision%29))
  (bind _questionmark (Variables|Default|GetQuestionMark))
  ;[0.15 0.15 0.15 0.5] Question Mark Face Camera & Translate
  (Utilities|FlowControl|Sequence
    (:then_0
      (if (Variables|Default|GetfaceCamera)
        (Utilities|IsValid (Variables|Default|GetQuestionMark)
          (:Is%20Valid
            (bind _returnvalue (Actor|GetActorOfClass "/Game/Hero/Blueprints/BP_ThirdPersonCharacter.BP_ThirdPersonCharacter_C"))
            (bind _location (Default|ReturnCameraLocation _returnvalue))
            (Transformation|SetActorRotation (Variables|Default|GetQuestionMark) (Math|Rotator|FindLookatRotation (Transformation|GetActorLocation (Variables|Default|GetQuestionMark)) _location))))))
    (:then_1
      (Utilities|IsValid _questionmark
        (:Is%20Valid
          (Transformation|SetActorLocation _questionmark (+ (Transformation|GetActorLocation) (Math|Vector|MakeVector 0.0 0.0 1.5e+02)) false false))))
    (:then_2
      ;[0.15 0.15 0.15 0.5] Excl Mark face cam
      (Utilities|IsValid (Variables|Default|GetExclamationMark)
        (:Is%20Valid
          (bind _returnvalue_2 (Actor|GetActorOfClass "/Game/Hero/Blueprints/BP_ThirdPersonCharacter.BP_ThirdPersonCharacter_C"))
          (bind _location_2 (Default|ReturnCameraLocation _returnvalue_2))
          (Transformation|SetActorRotation (Variables|Default|GetExclamationMark) (Math|Rotator|FindLookatRotation (Transformation|GetActorLocation (Variables|Default|GetExclamationMark)) _location_2)))))
    (:then_3
      (CallFunction|TranslateExclMark))
    (:then_4
      (CallFunction|PreferExclamationMark))))

(event Game|Damage|EventAnyDamage
  (params (Damage :type Float%20%28single-precision%29) (DamageType :type Damage%20Type%20Object%20Reference) (InstigatedBy :type Controller%20Object%20Reference) (DamageCauser :type Actor%20Object%20Reference))
  ;[0.15 0.15 0.15 0.5] Take damage
  (Development|PrintString "Took damage!")
  (bind _output_get (Variables|Default|SetHealth (Math|Float|Clamp(Float) (- (Variables|Default|GetHealth) Damage) 0.0 (Variables|Default|GetMaxHealth))))
  (if (<= _output_get 0.0)
    (Variables|Default|SetisDead? true)
    (else
      (Audio|PlaySoundatLocation "/Game/Audio/oof-97698.oof-97698" (Transformation|GetActorLocation) "0, 0, 0" 1.0 1.0 0.0 0 0 0 0))))

(fn ConstructionScript)

(fn Die
  (if (Variables|Default|GetallowDeathAnim)
    (Variables|Default|SetallowDeathAnim false)
    (Animation|Montage|MontagePlay (Components|SkeletalMesh|GetAnimInstance (Variables|Character|GetMesh)) "/Game/Enemies/Deputy/Anims/MON_Deputy_Death.MON_Deputy_Death" 1.0 "MontageLength" 0.0 true)
    (Collision|SetCollisionEnabled (Variables|Collision|GetCapsuleComponent) "NoCollision")
    (Audio|PlaySoundatLocation "/Game/Audio/man-death-scream-186763.man-death-scream-186763" (Transformation|GetActorLocation) "0, 0, 0" 1.0 1.0 0.0 0 0 0 0)
    (return true)
    (else
      (return true))))

(fn GetCurrentHealth
  (return (Variables|Default|GetHealth)))

(fn GetDistanceBetweenPoints
  (params (SourceVector :type Vector :default "0, 0, 0") (TargetVector :type Vector :default "0, 0, 0"))
  (bind _returnvalue (Game|GetPlayerCharacter 0))
  (bind _mesh (Variables|Character|GetMesh))
  (bind _mesh_2 (Variables|/Script/Engine.Character|GetMesh _returnvalue))
  (Utilities|IsValid _returnvalue
    (:Is%20Valid
      (Utilities|IsValid _mesh
        (:Is%20Valid
          (Utilities|IsValid _mesh_2
            (:Is%20Valid
              (return (Math|Vector|Distance(Vector) (Transformation|GetWorldLocation _mesh) (Transformation|GetWorldLocation _mesh_2))))
            (:Is%20Not%20Valid
              (Development|PrintString "Not valid!"))))
        (:Is%20Not%20Valid
          (Development|PrintString "Not valid!"))))))

(fn GetKOState
  (return (Variables|Default|GetisDead?)))

(fn Heal
  (params (HealAmount :type Float%20%28double-precision%29))
  (Variables|Default|SetHealth (Math|Float|Clamp(Float) (+ HealAmount (Variables|Default|GetHealth)) 0.0 (Variables|Default|GetMaxHealth)))
  (bind _asanim_bp_deputy (Utilities|Casting|CastToAnimBP_Deputy (Components|SkeletalMesh|GetAnimInstance (Variables|Character|GetMesh))))
  (Variables|/Game/Enemies/Deputy/AnimBP_Deputy.AnimBP_Deputy_C|SetisHealing? _asanim_bp_deputy true)
  (CallFunction|StopHeal)
  (return true))

(fn ReduceHealth
  (params (Damage :type Float%20%28double-precision%29)))

(fn SetMovementSpeed
  (params (Speed :type MoveSpeedState%20Enum :default "NewEnumerator0"))
  (bind _charactermovement (Variables|Character|GetCharacterMovement))
  (switch Utilities|FlowControl|Switch|SwitchonMoveSpeedState Speed
    (:NewEnumerator0
      (Variables|/Script/Engine.CharacterMovementComponent|SetMaxWalkSpeed _charactermovement 0.0))
    (:NewEnumerator1
      (Variables|/Script/Engine.CharacterMovementComponent|SetMaxWalkSpeed _charactermovement 1e+02))
    (:NewEnumerator2
      (Variables|/Script/Engine.CharacterMovementComponent|SetMaxWalkSpeed _charactermovement 2e+02))
    (:NewEnumerator3
      (Variables|/Script/Engine.CharacterMovementComponent|SetMaxWalkSpeed _charactermovement 3.2e+02)))
  (return (Variables|/Script/Engine.CharacterMovementComponent|GetMaxWalkSpeed _charactermovement)))

(fn ShowExclamationMark
  (bind _returnvalue (Game|SpawnActorfromClass "/Game/BluePrints/BP_Exclamation.BP_Exclamation_C" (Math|Transform|MakeTransform (+ (Transformation|GetActorLocation) (Math|Vector|MakeVector 0.0 0.0 1.5e+02)) "0, 0, 0" "1.000000,1.000000,1.000000") "Undefined" "MultiplyWithRoot" 0 0))
  (Variables|Default|SetExclamationMark _returnvalue)
  (CallFunction|DeleteExclamationMark)
  (return true))

(fn ShowQuestionMark
  (bind _returnvalue (Game|SpawnActorfromClass "/Game/BluePrints/BP_QuestionMark.BP_QuestionMark_C" (Math|Transform|MakeTransform (+ (Transformation|GetActorLocation) (Math|Vector|MakeVector 0.0 0.0 1.5e+02)) "0, 0, 0" "1.000000,1.000000,1.000000") "Undefined" "MultiplyWithRoot" 0 0))
  (Variables|Default|SetQuestionMark _returnvalue)
  (CallFunction|DeleteQuestionmark)
  (return true))