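; BP_Rifle is the hero's rifle actor, exposing a Fire event that shoots a projectile.
; Fire spawns a BP_Bullet at the Arrow component's transform, plays a gunshot sound and emits an AI noise event with the player pawn as instigator.
; It also attaches a Niagara muzzle flash to the Arrow and destroys it after a short delay.
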(event Custom|Fire
  (Game|SpawnActorfromClass "/Game/BluePrints/BP_Bullet.BP_Bullet_C" (Transformation|GetWorldTransform (Variables|Default|GetArrow)) "Undefined" "MultiplyWithRoot" 0 0)
  (Audio|PlaySoundatLocation "/Game/Audio/single-pistol-gunshot-33-37187.single-pistol-gunshot-33-37187" (Transformation|GetActorLocation) "0, 0, 0" 1.0 1.0 0.0 0 0 0 0)
  (Class|Actor|MakeNoise 1.0 (Game|Player|GetPlayerPawn 0) (Transformation|GetActorLocation) 1e+03 "None")
  (bind _returnvalue (Niagara|SpawnSystemAttached "/Game/VFX/Muzzle_Flash/FX/NS_Muzzle_Flash05.NS_Muzzle_Flash05" (Variables|Default|GetArrow) "None" "0, 0, 0" "0, 0, 0" "KeepRelativeOffset" false))
  (Utilities|FlowControl|Delay 0.4)
  (Components|DestroyComponent _returnvalue))

(event EventBeginPlay)

(event Collision|EventActorBeginOverlap
  (params (OtherActor :type Actor%20Object%20Reference)))

(event EventTick
  (params (DeltaSeconds :type Float%20%28single-precision%29)))

(fn ConstructionScript)