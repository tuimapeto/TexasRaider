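; Bank entrance door actor that rises with a turning gear and gear sound when its RaiseDoor event is called.
; The event sets a flag and spawns the sound, then stops both the sound and the motion after a fixed delay.
; While flagged, Tick eases world Z toward a fixed height with FInterpTo and spins the Gear component.
; World X and Y are hard-coded, tying the door to one level position.
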(event Custom|RaiseDoor
  ;[0.15 0.15 0.15 0.5] Raise Event & Sound
  (Variables|Default|SetraiseDoor? true)
  (bind _returnvalue (Audio|SpawnSoundatLocation "/Game/Audio/running-gear-6403.running-gear-6403" (Transformation|GetActorLocation) "0, 0, 0" 1.0 1.0 0.0 0 0))
  (Variables|Default|SetGearSound _returnvalue)
  (Utilities|FlowControl|Delay 3.0)
  (Audio|Components|Audio|Stop (Variables|Default|GetGearSound))
  (Variables|Default|SetraiseDoor? false))

(event EventBeginPlay
  ;[0.15 0.15 0.15 0.5] Raise Event & Sound
)

(event Collision|EventActorBeginOverlap
  (params (OtherActor :type Actor%20Object%20Reference)))

(event EventTick
  (params (DeltaSeconds :type Float%20%28single-precision%29))
  ;[0.15 0.15 0.15 0.5] Raise interpolation
  (if (Variables|Default|GetraiseDoor?)
    (Transformation|SetActorLocation (Math|Vector|MakeVector -6.793441 -1511.786196 (Math|Interpolation|FInterpTo (.Z (Math|Vector|BreakVector (Transformation|GetActorLocation))) 5e+02 DeltaSeconds 2.0)) false false)
    ;[0.15 0.15 0.15 0.5] Turn the Gear
    (bind _output_get (Variables|Default|SetTurnVar (+ (Variables|Default|GetTurnVar) (* (Variables|Default|GetTurnConst) DeltaSeconds))))
    (Transformation|SetWorldRotation (Variables|Default|GetGear) (Math|Rotator|MakeRotator 9e+01 _output_get 0.0) false false)))

(fn ConstructionScript)