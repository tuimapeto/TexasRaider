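; Key pickup actor that spins in yaw each tick at TurnAmount and is collected when BP_ThirdPersonCharacter overlaps its Key component.
; On first overlap it guards with IsAlreadyGot, increments the obtained keys on GM_Sequence and plays a pickup sound at world origin.
; It then spawns BP_ky_darkStorm 150 units below itself and destroys itself.
; A KeyBurst Niagara spawn node exists but is never run.
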(event OnComponentBeginOverlap(Key)
  (params (OverlappedComponent :type Primitive%20Component%20Object%20Reference) (OtherActor :type Actor%20Object%20Reference) (OtherComp :type Primitive%20Component%20Object%20Reference) (OtherBodyIndex :type Integer) (bFromSweep :type Boolean) (SweepResult :type Hit%20Result%20Structure%20%28by%20ref%29))
  (Utilities|Casting|CastToBP_ThirdPersonCharacter OtherActor)
  (if (not (Variables|Default|GetisAlreadyGot?))
    (Variables|Default|SetisAlreadyGot? true)
    (bind _asgm_sequence (Utilities|Casting|CastToGM_Sequence (Game|GetGameMode)))
    (Default|AddObtainedKeys _asgm_sequence)
    (Audio|PlaySoundatLocation "/Game/Audio/GetKeyNew.GetKeyNew" "0, 0, 0" "0, 0, 0" 1.0 1.0 0.0 0 0 0 0)
    (Game|SpawnActorfromClass "/Game/VFX/FXVarietyPack/Blueprints/BP_ky_darkStorm.BP_ky_darkStorm_C" (Math|Transform|MakeTransform (- (Transformation|GetActorLocation) "0.000000,0.000000,150.000000")) "Undefined" "MultiplyWithRoot" 0 0)
    (Actor|DestroyActor)))

(event EventTick
  (params (DeltaSeconds :type Float%20%28single-precision%29))
  (Transformation|AddActorLocalRotation (Math|Rotator|MakeRotator 0.0 0.0 (* DeltaSeconds (Variables|Default|GetturnAmount))) false false))

(fn ConstructionScript)