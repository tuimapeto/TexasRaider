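; BP_Beaver is a spinning beaver pelt pickup that the third-person player character collects.
; Tick rotates the actor in yaw at TurnSpeed, scaled by delta time.
; When the character overlaps BeaverPelt, a one-shot flag guards a call to increase the pelt count on GM_Sequence.
; It then plays a cash register sound at world origin and destroys itself.
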(event OnComponentBeginOverlap(BeaverPelt)
  (params (OverlappedComponent :type Primitive%20Component%20Object%20Reference) (OtherActor :type Actor%20Object%20Reference) (OtherComp :type Primitive%20Component%20Object%20Reference) (OtherBodyIndex :type Integer) (bFromSweep :type Boolean) (SweepResult :type Hit%20Result%20Structure%20%28by%20ref%29))
  ;[0.15 0.15 0.15 0.5] Increase the pelt number
  (Utilities|Casting|CastToBP_ThirdPersonCharacter OtherActor)
  (if (not (Variables|Default|GetIs%20Already%20Got?))
    (Variables|Default|SetIs%20Already%20Got? true)
    (bind _asgm_sequence (Utilities|Casting|CastToGM_Sequence (Game|GetGameMode)))
    (Default|IncreasePeltNumber _asgm_sequence)
    (Audio|PlaySoundatLocation "/Game/Audio/CashRegAud.CashRegAud" "0, 0, 0" "0, 0, 0" 1.0 1.0 0.0 0 0 0 0)
    (Actor|DestroyActor)))

(event EventBeginPlay)

(event Collision|EventActorBeginOverlap
  (params (OtherActor :type Actor%20Object%20Reference)))

(event EventTick
  (params (DeltaSeconds :type Float%20%28single-precision%29))
  ;[0.15 0.15 0.15 0.5] Rotate
  (Transformation|AddActorLocalRotation (Math|Rotator|MakeRotator 0.0 0.0 (* DeltaSeconds (Variables|Default|GetTurnSpeed))) false false))

(fn ConstructionScript)