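; BP_BulletBase is a base bullet that flies toward where the player character stood when the bullet spawned.
; BeginPlay takes the normalized direction to player 0, scales it to a fixed speed and applies a small fixed rotation offset.
; Tick writes that cached vector to the ProjectileMovement velocity every frame, so the bullet travels straight without homing.
; It contains no hit or damage logic.
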(event EventBeginPlay
  (Variables|Default|SetForwardVec (Math|Vector|RotateVector (* (Math|Vector|Normalize (- (Transformation|GetActorLocation (Game|GetPlayerCharacter 0)) (Transformation|GetActorLocation))) "100.000000,100.000000,100.000000") "0.000000,-5.000000,0.000000")))

(event Collision|EventActorBeginOverlap
  (params (OtherActor :type Actor%20Object%20Reference)))

(event EventTick
  (params (DeltaSeconds :type Float%20%28single-precision%29))
  (Variables|/Script/Engine.MovementComponent|SetVelocity (Variables|Default|GetProjectileMovement) (Variables|Default|GetForwardVec)))

(fn ConstructionScript)