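; Level game mode (GM_Sequence) that spawns the third-person hero, runs the bank entrance cutscene and tracks collected pelts and keys.
; BeginPlay uses timed delays to raise the door, play a walk montage, blend from a CameraActor to the hero camera, add LevelUI and possess the hero.
; Tick slides the hero inside by interpolating Y during the walk.
; Pelt and key events push counts to LevelUI; the exit-opening check is disconnected.
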(event Custom|AddObtainedKeys
  ;[0.15 0.15 0.15 0.5] Show keys on the screen
  (bind _result (Math|Integer|IncrementInt (Variables|Default|GetnumKeys))
    (:%20%20
      (Default|AddScoreText (Variables|Default|GetUserInterface) _result (Variables|Default|GetMaxKeys)))))

(event Custom|IncreasePeltNumber
  ;[0.15 0.15 0.15 0.5] Send pelt info to UI
  (bind _result (Math|Integer|IncrementInt (Variables|Default|GetNumberOfPelts))
    (:%20%20
      (Default|IncreasePelts (Variables|Default|GetUserInterface) _result)
      (Development|PrintString "More Pelts!"))))

(event Custom|MovePlayerINEntrance)

(event EventBeginPlay
  (bind _returnvalue (Game|GetPlayerController 0))
  ;[0.15 0.15 0.15 0.5] Initialize UI and Player
  (bind _returnvalue_2 (UserInterface|CreateWidget "/Game/UI/FadeUI.FadeUI_C"))
  (bind _output_get (Variables|Default|SetFadeScreen _returnvalue_2))
  (UserInterface|Viewport|AddtoViewport _output_get 0)
  (bind _returnvalue_3 (Game|SpawnActorfromClass "/Game/Hero/Blueprints/BP_ThirdPersonCharacter.BP_ThirdPersonCharacter_C" (Math|Transform|MakeTransform "-280.000000,-1700.000000,100.000000") "Undefined" "MultiplyWithRoot" 0 0))
  (Variables|Default|SetHero _returnvalue_3)
  ;[0.15 0.15 0.15 0.5] Entrance Cutscene
  (bind _outactors (Actor|GetAllActorsOfClass "/Script/Engine.CameraActor"))
  (Game|Player|SetViewTargetwithBlend (Game|GetPlayerController 0) (Utilities|Array|Get(acopy) _outactors) 0.0 "VTBlend_Linear" 0.0 false)
  (Utilities|FlowControl|Delay 2.0)
  (bind _outactors_2 (Actor|GetAllActorsOfClass "/Game/Objects/BankDoor/BP_BankEntranceDoor.BP_BankEntranceDoor_C"))
  (Default|RaiseDoor _outactors_2)
  (Transformation|SetActorRotation (Variables|Default|GetHero) "0.000000,90.000000,0.000000")
  (Utilities|FlowControl|Delay 2.0)
  (Variables|Default|SetmovePlayerInEntrance? true)
  (bind _asbp_blondie_anim (Utilities|Casting|CastToBP_BlondieAnim (Components|SkeletalMesh|GetAnimInstance (Variables|/Script/Engine.Character|GetMesh (Variables|Default|GetHero)))))
  (Variables|/Game/Hero/Blondie2/BP_BlondieAnim.BP_BlondieAnim_C|SetisCutSceneRunning? _asbp_blondie_anim true)
  (Animation|Montage|PlayMontage (Variables|/Script/Engine.Character|GetMesh (Variables|Default|GetHero)) "/Game/Retargeting/MONWalkNew_Blondie.MONWalkNew_Blondie"
    (:then
      (Utilities|FlowControl|Delay 2.06)
      (Animation|Montage|MontageStop (Components|SkeletalMesh|GetAnimInstance (Variables|/Script/Engine.Character|GetMesh (Variables|Default|GetHero))) 0.0 "/Game/Retargeting/MONWalkNew_Blondie.MONWalkNew_Blondie")
      (Variables|Default|SetmovePlayerInEntrance? false)
      (Development|PrintString (Utilities|String|ToString(Integer) (Utilities|Array|Length (Actor|GetComponentsbyTag (Variables|Default|GetHero) "/Script/Engine.CameraComponent" "MainCam"))))
      (Game|Player|SetViewTargetwithBlend _returnvalue (Components|GetOwner (Utilities|Array|Get(acopy) (Actor|GetComponentsbyTag (Variables|Default|GetHero) "/Script/Engine.CameraComponent" "MainCam"))) 3.0 "VTBlend_Linear" 0.0 false)
      (bind _returnvalue_4 (UserInterface|CreateWidget "/Game/UI/LevelUI.LevelUI_C"))
      (bind _output_get_2 (Variables|Default|SetUserInterface _returnvalue_4))
      (UserInterface|Viewport|AddtoViewport _output_get_2 0)
      (Utilities|FlowControl|Delay 2.0)
      (Default|StartMessageEvent _returnvalue_4)
      (Pawn|Possess _returnvalue (Variables|Default|GetHero)))))

(event EventTick
  (params (DeltaSeconds :type Float%20%28single-precision%29))
  (bind _hero (Variables|Default|GetHero))
  ;[0.15 0.15 0.15 0.5] Cutscene Movement
  (if (Variables|Default|GetmovePlayerInEntrance?)
    (Transformation|SetActorLocation _hero (Math|Vector|MakeVector -2.8e+02 (Math|Interpolation|FInterpTo (.Y (Math|Vector|BreakVector (Transformation|GetActorLocation _hero))) -1.4e+03 DeltaSeconds 1.0) 1e+02) false false)))

(fn ConstructionScript)