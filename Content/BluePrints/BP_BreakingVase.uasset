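; Breakable Chaos Geometry Collection vase that releases a BP_Beaver when it shatters.
; A hit from the third-person character or a bullet (which is destroyed) enables physics and break events, and spawns an FS_MasterField at the impact point.
; The break event makes debris ignore pawns, spawns one slightly raised beaver behind a once-only flag, then destroys the vase after a short delay.
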(event OnComponentHit(GC_Vase)
  (params (HitComponent :type Primitive%20Component%20Object%20Reference) (OtherActor :type Actor%20Object%20Reference) (OtherComp :type Primitive%20Component%20Object%20Reference) (NormalImpulse :type Vector :default "0, 0, 0") (Hit :type Hit%20Result%20Structure%20%28by%20ref%29))
  ;[0.15 0.15 0.15 0.5] Vase Break
  (Utilities|Casting|CastToBP_ThirdPersonCharacter OtherActor
    (:then
      _)
    (:CastFailed
      (bind _asbp_bullet (Utilities|Casting|CastToBP_Bullet OtherActor))
      (Actor|DestroyActor _asbp_bullet)))
  (Physics|SetSimulatePhysics (Variables|Default|GetGC_Vase) true)
  (Physics|SetEnableGravity (Variables|Default|GetGC_Vase) true)
  (Game|SpawnActorfromClass "/Engine/EditorResources/FieldNodes/FS_MasterField.FS_MasterField_C" (Math|Transform|MakeTransform (.Location (Collision|BreakHitResult Hit))) "Undefined" "MultiplyWithRoot" 0 0)
  (Class|GeometryCollectionComponent|SetNotifyBreaks (Variables|Default|GetGC_Vase) true))

(event OnComponentBeginOverlap(GC_Vase)
  (params (OverlappedComponent :type Primitive%20Component%20Object%20Reference) (OtherActor :type Actor%20Object%20Reference) (OtherComp :type Primitive%20Component%20Object%20Reference) (OtherBodyIndex :type Integer) (bFromSweep :type Boolean) (SweepResult :type Hit%20Result%20Structure%20%28by%20ref%29))
  ;[0.15 0.15 0.15 0.5] Vase Break
)

(event OnChaosBreakEvent(GC_Vase)
  (params (BreakEvent :type Chaos%20Break%20Event%20Structure%20%28by%20ref%29))
  ;[0.15 0.15 0.15 0.5] Vase Break
  (Collision|SetCollisionResponsetoChannel (Variables|Default|GetGC_Vase) "ECC_Pawn" "ECR_Ignore")
  (if (not (Variables|Default|GetisBeaverAlreadySpawned?))
    (bind _returnvalue (Game|SpawnActorfromClass "/Game/BluePrints/BP_Beaver.BP_Beaver_C" (Transformation|GetActorTransform) "Undefined" "MultiplyWithRoot" 0 0))
    (Variables|Default|SetisBeaverAlreadySpawned? true)
    (Utilities|IsValid _returnvalue
      (:Is%20Valid
        (Transformation|AddActorWorldOffset _returnvalue "0.000000,0.000000,50.000000"))
      (:Is%20Not%20Valid
        _))
    (Utilities|FlowControl|Delay 3.0)
    (Actor|DestroyActor)))

(event EventBeginPlay)

(event Collision|EventActorBeginOverlap
  (params (OtherActor :type Actor%20Object%20Reference)))

(event EventTick
  (params (DeltaSeconds :type Float%20%28single-precision%29)))

(fn ConstructionScript)